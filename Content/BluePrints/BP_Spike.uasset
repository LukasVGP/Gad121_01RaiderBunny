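; BP_Spike is a hazard that costs the third-person character a life on contact.
; On BeginPlay it binds to the KillZone overlap event, which casts the overlapping actor to BP_ThirdPersonCharacter and decrements Lives.
; If lives remain, the character moves back to its stored PlayerStartLocation.
; Nothing happens here at zero lives; the viewport widget and pause nodes are unconnected.
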(event Custom|OnComponentBeginOverlap_Event
  (params (OverlappedComponent :type Primitive%20Component%20Object%20Reference) (OtherActor :type Actor%20Object%20Reference) (OtherComp :type Primitive%20Component%20Object%20Reference) (OtherBodyIndex :type Integer) (bFromSweep :type Boolean) (SweepResult :type Hit%20Result%20Structure%20%28by%20ref%29))
  (bind _asbp_third_person_character (Utilities|Casting|CastToBP_ThirdPersonCharacter OtherActor))
  (bind _output_get (Variables|/Game/ThirdPerson/Blueprints/BP_ThirdPersonCharacter.BP_ThirdPersonCharacter_C|SetLives _asbp_third_person_character (- (Variables|/Game/ThirdPerson/Blueprints/BP_ThirdPersonCharacter.BP_ThirdPersonCharacter_C|GetLives _asbp_third_person_character) 1)))
  (if (> _output_get 0)
    (Transformation|SetActorLocation _asbp_third_person_character (Variables|/Game/ThirdPerson/Blueprints/BP_ThirdPersonCharacter.BP_ThirdPersonCharacter_C|GetPlayerStartLocation _asbp_third_person_character) false false)))

(event EventBeginPlay
  (Collision|AssignOnComponentBeginOverlap (Variables|Default|GetKillZone) (delegate Custom|OnComponentBeginOverlap_Event)))

(fn ConstructionScript)