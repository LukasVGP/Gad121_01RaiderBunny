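; BP_Checkpoint is a pickup-style checkpoint that moves the player's start location to its own position.
; Until activated, its pyramid mesh spins around the yaw axis on Tick at a constant, frame-rate-independent speed.
; When a BP_ThirdPersonCharacter overlaps it, it writes its location to that character's PlayerStartLocation, sets Activated, then hides itself and disables collision.
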(event EventBeginPlay)

(event Collision|EventActorBeginOverlap
  (params (OtherActor :type Actor%20Object%20Reference))
  (bind _asbp_third_person_character (Utilities|Casting|CastToBP_ThirdPersonCharacter OtherActor))
  (Variables|Default|SetbActivated true)
  (Variables|/Game/ThirdPerson/Blueprints/BP_ThirdPersonCharacter.BP_ThirdPersonCharacter_C|SetPlayerStartLocation _asbp_third_person_character (Transformation|GetActorLocation))
  (Rendering|SetActorHiddenInGame true)
  (Collision|SetActorEnableCollision false))

(event EventTick
  (params (DeltaSeconds :type Float%20%28single-precision%29))
  (if (not (Variables|Default|GetbActivated))
    (Transformation|AddLocalRotation (Variables|Default|GetPyramidMesh) (Math|Rotator|MakeRotator 0.0 0.0 (* DeltaSeconds 9e+01)) false false)))

(fn ConstructionScript)