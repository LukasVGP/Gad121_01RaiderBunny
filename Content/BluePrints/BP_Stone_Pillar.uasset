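; BP_Stone_Pillar is a stone pillar that moves back and forth continuously between two points.
; Tick ramps MoveAlpha up or down and lerps PillarMesh's relative location from StartPoint to EndPoint, reversing MovingForward at either end.
; MoveSpeed divides delta time, so it acts as seconds per one-way trip rather than a speed.
; The construction script places the mesh at StartPoint.
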(event EventBeginPlay)

(event Collision|EventActorBeginOverlap
  (params (OtherActor :type Actor%20Object%20Reference)))

(event EventTick
  (params (DeltaSeconds :type Float%20%28single-precision%29))
  (if (Variables|Default|GetbMovingForward)
    (Variables|Default|SetMoveAlpha (Math|Float|Clamp(Float) (+ (Variables|Default|GetMoveAlpha) (/ DeltaSeconds (Variables|Default|GetMoveSpeed)))))
    (else
      (Variables|Default|SetMoveAlpha (Math|Float|Clamp(Float) (- (Variables|Default|GetMoveAlpha) (/ DeltaSeconds (Variables|Default|GetMoveSpeed)))))))
  (Transformation|SetRelativeLocation (Variables|Default|GetPillarMesh) (Math|Vector|Lerp(Vector) (Variables|Default|GetStartPoint) (Variables|Default|GetEndPoint) (Variables|Default|GetMoveAlpha)) false false)
  (if (and (>= (Variables|Default|GetMoveAlpha) 1.0) (Variables|Default|GetbMovingForward))
    (Variables|Default|SetbMovingForward false))
  (if (and (<= (Variables|Default|GetMoveAlpha) 0.0) (not (Variables|Default|GetbMovingForward)))
    (Variables|Default|SetbMovingForward true)))

(fn ConstructionScript
  (Transformation|SetRelativeLocation (Variables|Default|GetPillarMesh) (Variables|Default|GetStartPoint) false false))