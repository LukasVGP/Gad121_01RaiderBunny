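; Basic interactable door that the third-person character triggers with the E key.
; TriggerZone overlap enables input and shows PromptText, and leaving it disables input and hides the prompt.
; E passes a never-reset DoOnce, plays a sound, and runs a Timeline that sets the Door's relative rotation.
; The rotator shown is constant zero, with no Timeline output feeding it.
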(event Custom|OnComponentBeginOverlap_Event
  (params (OverlappedComponent :type Primitive%20Component%20Object%20Reference) (OtherActor :type Actor%20Object%20Reference) (OtherComp :type Primitive%20Component%20Object%20Reference) (OtherBodyIndex :type Integer) (bFromSweep :type Boolean) (SweepResult :type Hit%20Result%20Structure%20%28by%20ref%29))
  (Utilities|Casting|CastToBP_ThirdPersonCharacter OtherActor)
  (Input|EnableInput (Game|GetPlayerController 0))
  (Development|SetHiddeninGame (Variables|Default|GetPromptText) false false))

(event Custom|OnComponentEndOverlap_Event
  (params (OverlappedComponent :type Primitive%20Component%20Object%20Reference) (OtherActor :type Actor%20Object%20Reference) (OtherComp :type Primitive%20Component%20Object%20Reference) (OtherBodyIndex :type Integer))
  (Utilities|Casting|CastToBP_ThirdPersonCharacter OtherActor)
  (Input|DisableInput (Game|GetPlayerController 0))
  (Development|SetHiddeninGame (Variables|Default|GetPromptText) true false))

(event EventBeginPlay
  (Collision|AssignOnComponentBeginOverlap (Variables|Default|GetTriggerZone) (delegate Custom|OnComponentBeginOverlap_Event))
  (Collision|AssignOnComponentEndOverlap (Variables|Default|GetTriggerZone) (delegate Custom|OnComponentEndOverlap_Event)))

(event Collision|EventActorBeginOverlap
  (params (OtherActor :type Actor%20Object%20Reference)))

(event EventTick
  (params (DeltaSeconds :type Float%20%28single-precision%29)))

(event Input|KeyboardEvents|E
  (params (Key :type Key%20Structure))
  (:Pressed
    (Utilities|FlowControl|DoOnce false
      (:Completed
        (Audio|PlaySoundatLocation 0 (Transformation|GetActorLocation) "0, 0, 0" 1.0 1.0 0.0 0 0 0 0)
        (Timeline|Timeline Play
          (:Update
            (Transformation|SetRelativeRotation (Variables|Default|GetDoor) (Math|Rotator|MakeRotator 0.0 0.0 0.0) false false)))))))

(fn ConstructionScript)