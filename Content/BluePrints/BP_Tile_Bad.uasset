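; BP_Tile_Bad is a trap tile that shakes and falls when the player character steps on it, then respawns.
; An overlap on TileTrigger passes a DoOnce, plays a sound and jitters TileMesh with chained Delays before enabling physics to drop it.
; After a pause it hides, returns to the location saved at BeginPlay, waits, then reappears, re-enabling the trigger and resetting the DoOnce.
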(event Custom|OnTileTrigger_Overlap
  (params (OverlappedComponent :type Primitive%20Component%20Object%20Reference) (OtherActor :type Actor%20Object%20Reference) (OtherComp :type Primitive%20Component%20Object%20Reference) (OtherBodyIndex :type Integer) (bFromSweep :type Boolean) (SweepResult :type Hit%20Result%20Structure))
  (Utilities|Casting|CastToBP_ThirdPersonCharacter (stale Custom|OnComponentBeginOverlap_Event_0 OtherActor))
  (Utilities|FlowControl|DoOnce false :!label _label
    (:Completed
      (Audio|PlaySoundatLocation 0 (Transformation|GetActorLocation) "0, 0, 0" 1.0 1.0 0.0 0 0 0 0)
      (Transformation|SetRelativeLocation (Variables|Default|GetTileMesh) "(X=10,Y=0,Z=0)" false false)
      (Utilities|FlowControl|Delay 0.12)
      (Transformation|SetRelativeLocation (Variables|Default|GetTileMesh) "(X=-10,Y=0,Z=0)" false false)
      (Utilities|FlowControl|Delay 0.12)
      (Transformation|SetRelativeLocation (Variables|Default|GetTileMesh) "(X=10,Y=0,Z=0)" false false)
      (Utilities|FlowControl|Delay 0.12)
      (Transformation|SetRelativeLocation (Variables|Default|GetTileMesh) "(X=-10,Y=0,Z=0)" false false)
      (Utilities|FlowControl|Delay 0.12)
      (Transformation|SetRelativeLocation (Variables|Default|GetTileMesh) "(X=10,Y=0,Z=0)" false false)
      (Utilities|FlowControl|Delay 0.12)
      (Transformation|SetRelativeLocation (Variables|Default|GetTileMesh) "(X=-10,Y=0,Z=0)" false false)
      (Utilities|FlowControl|Delay 0.12)
      (Transformation|SetRelativeLocation (Variables|Default|GetTileMesh) "0, 0, 0" false false)
      (Physics|SetSimulatePhysics (Variables|Default|GetTileMesh) true)
      (Collision|SetCollisionEnabled (Variables|Default|GetTileTrigger) "NoCollision")
      (Utilities|FlowControl|Delay 3.0)
      (Rendering|SetActorHiddenInGame true)
      (Physics|SetSimulatePhysics (Variables|Default|GetTileMesh) false)
      (Transformation|SetRelativeLocation (Variables|Default|GetTileMesh) "0, 0, 0" false false)
      (Transformation|SetActorLocation (Variables|Default|GetInitialLocation) false false)
      (Utilities|FlowControl|Delay 15.0)
      (Rendering|SetActorHiddenInGame false)
      (Collision|SetCollisionEnabled (Variables|Default|GetTileTrigger) "QueryOnly")
      (goto _label Reset))))

(event Custom|OnComponentBeginOverlap_Event_0
  (params (OverlappedComponent :type Primitive%20Component%20Object%20Reference) (OtherActor :type Actor%20Object%20Reference) (OtherComp :type Primitive%20Component%20Object%20Reference) (OtherBodyIndex :type Integer) (bFromSweep :type Boolean) (SweepResult :type Hit%20Result%20Structure%20%28by%20ref%29))
  (Utilities|Casting|CastToBP_ThirdPersonCharacter OtherActor)
  (Utilities|FlowControl|DoOnce false :!label _label
    (:Completed
      (Audio|PlaySoundatLocation 0 (Transformation|GetActorLocation) "0, 0, 0" 1.0 1.0 0.0 0 0 0 0)
      (Transformation|SetRelativeLocation (Variables|Default|GetTileMesh) "(X=10,Y=0,Z=0)" false false)
      (Utilities|FlowControl|Delay 0.12)
      (Transformation|SetRelativeLocation (Variables|Default|GetTileMesh) "(X=-10,Y=0,Z=0)" false false)
      (Utilities|FlowControl|Delay 0.12)
      (Transformation|SetRelativeLocation (Variables|Default|GetTileMesh) "(X=10,Y=0,Z=0)" false false)
      (Utilities|FlowControl|Delay 0.12)
      (Transformation|SetRelativeLocation (Variables|Default|GetTileMesh) "(X=-10,Y=0,Z=0)" false false)
      (Utilities|FlowControl|Delay 0.12)
      (Transformation|SetRelativeLocation (Variables|Default|GetTileMesh) "(X=10,Y=0,Z=0)" false false)
      (Utilities|FlowControl|Delay 0.12)
      (Transformation|SetRelativeLocation (Variables|Default|GetTileMesh) "(X=-10,Y=0,Z=0)" false false)
      (Utilities|FlowControl|Delay 0.12)
      (Transformation|SetRelativeLocation (Variables|Default|GetTileMesh) "0, 0, 0" false false)
      (Physics|SetSimulatePhysics (Variables|Default|GetTileMesh) true)
      (Collision|SetCollisionEnabled (Variables|Default|GetTileTrigger) "NoCollision")
      (Utilities|FlowControl|Delay 3.0)
      (Rendering|SetActorHiddenInGame true)
      (Physics|SetSimulatePhysics (Variables|Default|GetTileMesh) false)
      (Transformation|SetRelativeLocation (Variables|Default|GetTileMesh) "0, 0, 0" false false)
      (Transformation|SetActorLocation (Variables|Default|GetInitialLocation) false false)
      (Utilities|FlowControl|Delay 15.0)
      (Rendering|SetActorHiddenInGame false)
      (Collision|SetCollisionEnabled (Variables|Default|GetTileTrigger) "QueryOnly")
      (goto _label Reset))))

(event EventBeginPlay
  (Collision|AssignOnComponentBeginOverlap (Variables|Default|GetTileTrigger) (delegate Custom|OnComponentBeginOverlap_Event_0))
  (Variables|Default|SetInitialLocation (Transformation|GetActorLocation)))

(event Collision|EventActorBeginOverlap
  (params (OtherActor :type Actor%20Object%20Reference)))

(event EventTick
  (params (DeltaSeconds :type Float%20%28single-precision%29)))

(fn ConstructionScript)