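; BP_CaveTorch is a cave torch actor whose light flickers like a flame.
; On BeginPlay a looping timer calls UpdateFlicker at short intervals to pick a random target intensity.
; Tick eases the current intensity toward that target with FInterpTo and applies it to TorchLight, smoothing the random jumps.
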(event Custom|UpdateFlicker
  (Variables|Default|SetTargetIntensity (Math|Random|RandomFloatinRange 8e+02 2e+03)))

(event EventBeginPlay
  (Utilities|Time|SetTimerbyFunctionName 0 "UpdateFlicker" 0.07 true))

(event Collision|EventActorBeginOverlap
  (params (OtherActor :type Actor%20Object%20Reference)))

(event EventTick
  (params (DeltaSeconds :type Float%20%28single-precision%29))
  (bind _output_get (Variables|Default|SetCurrentIntensity (Math|Interpolation|FInterpTo (Variables|Default|GetCurrentIntensity) (Variables|Default|GetTargetIntensity) DeltaSeconds 8.0)))
  (Rendering|Components|Light|SetIntensity (Variables|Default|GetTorchLight) _output_get))

(fn ConstructionScript)