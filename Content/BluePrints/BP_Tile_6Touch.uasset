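; BP_Tile_6Touch is a tile actor that destroys itself after six touches.
; On BeginPlay it binds a handler to the TileTrigger begin-overlap event.
; Each overlap calls play-sound at the tile's location and increments TouchCount, destroying the actor once the count reaches six, with no filter on the overlapping actor.
; A second overlap handler is empty and its binding never runs.
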(event Custom|OnComponentBeginOverlap_Event
  (params (OverlappedComponent :type Primitive%20Component%20Object%20Reference) (OtherActor :type Actor%20Object%20Reference) (OtherComp :type Primitive%20Component%20Object%20Reference) (OtherBodyIndex :type Integer) (bFromSweep :type Boolean) (SweepResult :type Hit%20Result%20Structure%20%28by%20ref%29)))

(event Custom|OnComponentBeginOverlap_Event_0
  (params (OverlappedComponent :type Primitive%20Component%20Object%20Reference) (OtherActor :type Actor%20Object%20Reference) (OtherComp :type Primitive%20Component%20Object%20Reference) (OtherBodyIndex :type Integer) (bFromSweep :type Boolean) (SweepResult :type Hit%20Result%20Structure%20%28by%20ref%29))
  (Audio|PlaySoundatLocation 0 (Transformation|GetActorLocation) "0, 0, 0" 1.0 1.0 0.0 0 0 0 0)
  (Variables|Default|SetTouchCount (+ (Variables|Default|GetTouchCount) 1))
  (if (>= (Variables|Default|GetTouchCount) 6)
    (Actor|DestroyActor)))

(event EventBeginPlay
  (Collision|AssignOnComponentBeginOverlap (Variables|Default|GetTileTrigger) (delegate Custom|OnComponentBeginOverlap_Event_0)))

(event Collision|EventActorBeginOverlap
  (params (OtherActor :type Actor%20Object%20Reference)))

(event EventTick
  (params (DeltaSeconds :type Float%20%28single-precision%29)))

(fn ConstructionScript)