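; Falling spike trap that drops when its trigger zone is overlapped and costs the player a life on kill zone contact.
; Tick lowers the spike mesh from SpikeHeight, playing sounds at trigger and landing, then raises it after a delay.
; A DoOnce blocks retriggering until the spikes are fully raised.
; KillPlayer returns the third-person character to its start, or shows the lose menu and pauses when lives run out.
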(event Custom|OnKillZone_BeginOverlap
  (params (OtherActor :type Actor%20Object%20Reference) (OverlappedComponent :type Primitive%20Component%20Object%20Reference) (OtherComp :type Primitive%20Component%20Object%20Reference) (OtherBodyIndex :type Integer) (bFromSweep :type Boolean) (SweepResult :type Hit%20Result%20Structure))
  (CallFunction|KillPlayer OtherActor))

(event Custom|OnTriggerZone_BeginOverlap
  (params (OtherActor :type Actor%20Object%20Reference) (OverlappedComponent :type Primitive%20Component%20Object%20Reference) (OtherComp :type Primitive%20Component%20Object%20Reference) (OtherBodyIndex :type Integer) (bFromSweep :type Boolean) (SweepResult :type Hit%20Result%20Structure))
  (Utilities|FlowControl|DoOnce false))

(event Custom|OnComponentBeginOverlap_Event
  (params (OverlappedComponent :type Primitive%20Component%20Object%20Reference) (OtherActor :type Actor%20Object%20Reference) (OtherComp :type Primitive%20Component%20Object%20Reference) (OtherBodyIndex :type Integer) (bFromSweep :type Boolean) (SweepResult :type Hit%20Result%20Structure%20%28by%20ref%29)))

(event Custom|OnComponentBeginOverlap_Event_0
  (params (OverlappedComponent :type Primitive%20Component%20Object%20Reference) (OtherActor :type Actor%20Object%20Reference) (OtherComp :type Primitive%20Component%20Object%20Reference) (OtherBodyIndex :type Integer) (bFromSweep :type Boolean) (SweepResult :type Hit%20Result%20Structure%20%28by%20ref%29)))

(event Custom|OnKillZone_Overlap
  (params (OverlappedComponent :type Primitive%20Component%20Object%20Reference) (OtherActor :type Actor%20Object%20Reference) (OtherComp :type Primitive%20Component%20Object%20Reference) (OtherBodyIndex :type Integer) (bFromSweep :type Boolean) (SweepResult :type Hit%20Result%20Structure%20%28by%20ref%29))
  (CallFunction|KillPlayer OtherActor))

(event Custom|OnTriggerZone_Overlap
  (params (OverlappedComponent :type Primitive%20Component%20Object%20Reference) (OtherActor :type Actor%20Object%20Reference) (OtherComp :type Primitive%20Component%20Object%20Reference) (OtherBodyIndex :type Integer) (bFromSweep :type Boolean) (SweepResult :type Hit%20Result%20Structure%20%28by%20ref%29))
  (Utilities|FlowControl|DoOnce false
    (:Completed
      (Audio|PlaySoundatLocation (Variables|Audio|GetExplosionSound) (Transformation|GetActorLocation) "0, 0, 0" 1.0 1.0 0.0 0 0 0 0)
      (Variables|Default|SetbIsFalling true))))

(event EventBeginPlay
  (Collision|AssignOnComponentBeginOverlap (Variables|Default|GetKillZone) (delegate Custom|OnKillZone_Overlap))
  (Collision|AssignOnComponentBeginOverlap (Variables|Default|GetTriggerZone) (delegate Custom|OnTriggerZone_Overlap)))

(event Collision|EventActorBeginOverlap
  (params (OtherActor :type Actor%20Object%20Reference)))

(event EventTick
  (params (DeltaSeconds :type Float%20%28single-precision%29))
  (bind _fallspeed (Variables|Default|GetFallSpeed))
  (bind _spikeheight (Variables|Default|GetSpikeHeight))
  (bind _spikemesh (Variables|Default|GetSpikeMesh))
  (bind _spikemesh_2 (Variables|Default|GetSpikeMesh))
  (bind _returnvalue (* _fallspeed DeltaSeconds))
  (bind _relativelocation (Variables|/Script/Engine.SceneComponent|GetRelativeLocation _spikemesh))
  (bind _relativelocation_2 (Variables|/Script/Engine.SceneComponent|GetRelativeLocation _spikemesh_2))
  (bind _z (Math|Vector|BreakVector _relativelocation_2))
  (bind _z_2 (Math|Vector|BreakVector _relativelocation))
  (bind _returnvalue_2 (- _z _returnvalue))
  (bind _returnvalue_3 (+ _z_2 _returnvalue))
  (bind _returnvalue_4 (Math|Float|Clamp(Float) _returnvalue_3 0.0 _spikeheight))
  (bind _returnvalue_5 (Math|Float|Clamp(Float) _returnvalue_2 0.0 _spikeheight))
  (if (Variables|Default|GetbIsFalling)
    (Transformation|SetRelativeLocation (Variables|Default|GetSpikeMesh) (Math|Vector|MakeVector 0.0 0.0 _returnvalue_5) false false)
    (if (<= _returnvalue_5 0.0)
      (Variables|Default|SetbIsFalling false)
      (Audio|PlaySoundatLocation (Variables|Audio|GetExplosionSound) (Transformation|GetActorLocation) "0, 0, 0" 1.0 1.0 0.0 0 0 0 0)
      (Utilities|FlowControl|Delay 1e+01)
      (Variables|Default|SetbIsRising true))
    (elif (Variables|Default|GetbIsRising)
      (Transformation|SetRelativeLocation (Variables|Default|GetSpikeMesh) (Math|Vector|MakeVector 0.0 0.0 _returnvalue_4) false false)
      (if (>= _returnvalue_4 _spikeheight)
        (Variables|Default|SetbIsRising false)
        (Utilities|FlowControl|DoOnce false) ; enters at Reset
      ))))

(fn ConstructionScript
  (Transformation|SetRelativeLocation (Variables|Default|GetSpikeMesh) (Math|Vector|MakeVector 0.0 0.0 (Variables|Default|GetSpikeHeight)) false false))

(fn KillPlayer
  (params (HitActor :type Actor%20Object%20Reference))
  (bind _asbp_third_person_character (Utilities|Casting|CastToBP_ThirdPersonCharacter HitActor))
  (bind _output_get (Variables|/Game/ThirdPerson/Blueprints/BP_ThirdPersonCharacter.BP_ThirdPersonCharacter_C|SetLives _asbp_third_person_character (- (Variables|/Game/ThirdPerson/Blueprints/BP_ThirdPersonCharacter.BP_ThirdPersonCharacter_C|GetLives _asbp_third_person_character) 1)))
  (if (> _output_get 0)
    (Transformation|SetActorLocation _asbp_third_person_character (Variables|/Game/ThirdPerson/Blueprints/BP_ThirdPersonCharacter.BP_ThirdPersonCharacter_C|GetPlayerStartLocation _asbp_third_person_character) false false)
    (Physics|SetPhysicsLinearVelocity (Variables|/Script/Engine.MovementComponent|GetUpdatedPrimitive (Variables|/Script/Engine.Character|GetCharacterMovement _asbp_third_person_character)) "0, 0, 0" false "None")
    (else
      (bind _returnvalue (UserInterface|CreateWidget "/Game/UI/LoseMenu_WBP.LoseMenu_WBP_C"))
      (UserInterface|Viewport|AddtoViewport _returnvalue 0)
      (Game|SetGamePaused true))))