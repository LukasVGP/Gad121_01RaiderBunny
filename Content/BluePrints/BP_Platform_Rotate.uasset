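; BP_Platform_Rotate is a platform that spins around its local yaw axis while the third-person character is inside its OverlapDetector.
; Overlap begin and end events, bound on BeginPlay, toggle IsRotating for BP_ThirdPersonCharacter only.
; Tick applies RotationSpeed scaled by delta time as local rotation while that flag is set.
; An angle-limit branch using CurrentRotation and RotationAngle is disconnected, so rotation has no limit.
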(event Custom|OnComponentBeginOverlap_Event
  (params (OverlappedComponent :type Primitive%20Component%20Object%20Reference) (OtherActor :type Actor%20Object%20Reference) (OtherComp :type Primitive%20Component%20Object%20Reference) (OtherBodyIndex :type Integer) (bFromSweep :type Boolean) (SweepResult :type Hit%20Result%20Structure%20%28by%20ref%29))
  (Utilities|Casting|CastToBP_ThirdPersonCharacter OtherActor)
  (Variables|PlatformSettings|SetbIsRotating true)
  (Variables|PlatformSettings|SetCurrentRotation 0.0))

(event Custom|OnOverlapDetectorEndOverlap
  (params (OverlappedComponent :type Primitive%20Component%20Object%20Reference) (OtherActor :type Actor%20Object%20Reference) (OtherComp :type Primitive%20Component%20Object%20Reference) (OtherBodyIndex :type Integer))
  (Utilities|Casting|CastToBP_ThirdPersonCharacter OtherActor)
  (Variables|PlatformSettings|SetbIsRotating false))

(event EventBeginPlay
  (Collision|AssignOnComponentBeginOverlap (Variables|Default|GetOverlapDetector) (delegate Custom|OnComponentBeginOverlap_Event))
  (Collision|AssignOnComponentEndOverlap (Variables|Default|GetOverlapDetector) (delegate Custom|OnOverlapDetectorEndOverlap)))

(event Collision|EventActorBeginOverlap
  (params (OtherActor :type Actor%20Object%20Reference)))

(event EventTick
  (params (DeltaSeconds :type Float%20%28single-precision%29))
  (if (Variables|PlatformSettings|GetbIsRotating)
    (Transformation|AddActorLocalRotation (Math|Rotator|MakeRotator 0.0 0.0 (* (Variables|PlatformSettings|GetRotationSpeed) DeltaSeconds)) false false)))

(fn ConstructionScript)