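; BP_FogZone is a trigger volume that changes height fog density and fades fog audio as BP_ThirdPersonCharacter enters or leaves.
; The construction script creates the overlap box and a silent, non-auto-activating audio component.
; BeginPlay caches the referenced fog component's original density.
; Overlap events play or reverse a timeline, whose normalized playback position blends from original to target density, while fading the sound in or out.
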(event EventBeginPlay
  (Variables|FogZone|SetFogComponentRef (Variables|/Script/Engine.ExponentialHeightFog|GetComponent (Variables|FogZone|GetHeightFogActor)))
  (Variables|FogZone|SetOriginalFogDensity (Variables|/Script/Engine.ExponentialHeightFogComponent|GetFogDensity (Variables|FogZone|GetFogComponentRef))))

(event Collision|EventActorBeginOverlap
  (params (OtherActor :type Actor%20Object%20Reference))
  (bind _timeline_0 (Variables|Default|GetTimeline_0))
  (Utilities|Casting|CastToBP_ThirdPersonCharacter OtherActor)
  (Utilities|FlowControl|Sequence
    (:then_0
      (Timeline|Timeline_0 Play
        (:Update
          (Class|ExponentialHeightFogComponent|SetFogDensity (Variables|FogZone|GetFogComponentRef) (Math|Float|Lerp (Variables|FogZone|GetOriginalFogDensity) (Variables|FogZone|GetFogDensity) (Math|Float|SafeDivide (Components|Timeline|GetPlaybackPosition _timeline_0) (Components|Timeline|GetTimelineLength _timeline_0)))))))
    (:then_1
      (Audio|Components|Audio|FadeIn (Variables|Components|GetAudioCompRef) (Variables|FogZone|GetSoundFadeTime) 1.0 0.0 "Linear" :!class /Script/Engine.AudioComponent))))

(event EventTick
  (params (DeltaSeconds :type Float%20%28single-precision%29)))

(event Collision|EventActorEndOverlap
  (params (OtherActor :type Actor%20Object%20Reference))
  (bind _timeline_0 (Variables|Default|GetTimeline_0))
  (Utilities|Casting|CastToBP_ThirdPersonCharacter OtherActor)
  (Utilities|FlowControl|Sequence
    (:then_0
      (Timeline|Timeline_0 Reverse
        (:Update
          (Class|ExponentialHeightFogComponent|SetFogDensity (Variables|FogZone|GetFogComponentRef) (Math|Float|Lerp (Variables|FogZone|GetOriginalFogDensity) (Variables|FogZone|GetFogDensity) (Math|Float|SafeDivide (Components|Timeline|GetPlaybackPosition _timeline_0) (Components|Timeline|GetTimelineLength _timeline_0)))))))
    (:then_1
      (Audio|Components|Audio|FadeOut (Variables|Components|GetAudioCompRef) (Variables|FogZone|GetSoundFadeTime) 0.0 "Linear" :!class /Script/Engine.AudioComponent))))

(fn ConstructionScript
  (bind _returnvalue (AddComponent|AddBoxComponent false))
  (Components|Box|SetBoxExtent _returnvalue "(X=600,Y=600,Z=400)" true)
  (Collision|SetCollisionProfileName _returnvalue "OverlapAllDynamic" true :!class /Script/Engine.PrimitiveComponent)
  (Class|PrimitiveComponent|SetGenerateOverlapEvents _returnvalue true)
  (bind _returnvalue_2 (AddComponent|AddAudioComponent false))
  (Audio|Components|Audio|SetSound _returnvalue_2 (Variables|Audio|GetFogSound))
  (Components|Activation|SetAutoActivate _returnvalue_2 false)
  (Variables|/Script/Engine.AudioComponent|SetVolumeMultiplier _returnvalue_2 0.0)
  (Variables|Components|SetAudioCompRef _returnvalue_2))