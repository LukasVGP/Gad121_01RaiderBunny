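; Crushing-walls trap that slams two meshes together when the player character overlaps the actor.
; A timeline lerps both walls inward along Y, pauses and reverses, repeating for five cycles before the DoOnce re-arms the trigger.
; Kill-zone overlaps call KillPlayer, which deducts a life and teleports the character to its start location, or shows HUD_WBP and pauses the game when none remain.
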(event Custom|OnComponentBeginOverlap_Event
  (params (OverlappedComponent :type Primitive%20Component%20Object%20Reference) (OtherActor :type Actor%20Object%20Reference) (OtherComp :type Primitive%20Component%20Object%20Reference) (OtherBodyIndex :type Integer) (bFromSweep :type Boolean) (SweepResult :type Hit%20Result%20Structure%20%28by%20ref%29))
  (CallFunction|KillPlayer OtherActor))

(event Custom|OnKillZone2BeginOverlap
  (params (OverlappedComponent :type Primitive%20Component%20Object%20Reference) (OtherActor :type Actor%20Object%20Reference) (OtherComp :type Primitive%20Component%20Object%20Reference) (OtherBodyIndex :type Integer) (bFromSweep :type Boolean) (SweepResult :type Hit%20Result%20Structure%20%28by%20ref%29))
  (CallFunction|KillPlayer OtherActor))

(event Custom|OnPistonHit
  (params (OtherActor :type Actor%20Object%20Reference))
  (CallFunction|KillPlayer OtherActor))

(event EventBeginPlay
  (Components|Timeline|SetPlayRate (Variables|Default|GetTimeline_1) (Variables|Default|GetSmashSpeed))
  (Collision|AssignOnComponentBeginOverlap (Variables|Default|GetKillZone1) (delegate Custom|OnComponentBeginOverlap_Event))
  (Collision|AssignOnComponentBeginOverlap (Variables|Default|GetKillZone2) (delegate Custom|OnKillZone2BeginOverlap)))

(event Collision|EventActorBeginOverlap
  (params (OtherActor :type Actor%20Object%20Reference))
  (bind _wallretractdistance (Variables|Default|GetWallRetractDistance))
  (Utilities|Casting|CastToBP_ThirdPersonCharacter OtherActor)
  (Utilities|FlowControl|DoOnce false :!label _label
    (:Completed
      (Variables|Default|SetCrushCycleCount 0)
      (Audio|PlaySoundatLocation (Variables|Audio|GetCrushSound) (Transformation|GetActorLocation) "0, 0, 0" 1.0 1.0 0.0 0 0 0 0)
      (bind _newtrack_0 (Timeline|Timeline_1 PlayFromStart)
        (:Update
          (Transformation|SetRelativeLocation (Variables|Default|GetCrushMesh01) (Math|Vector|MakeVector 0.0 (Math|Float|Lerp _wallretractdistance 0.0 (Math|Float|SafeDivide _newtrack_0 5.0)) 0.0) false false)
          (bind _sweephitresult (Transformation|SetRelativeLocation (Variables|Default|GetCrushMesh02) (Math|Vector|MakeVector 0.0 (Math|Float|Lerp (* _wallretractdistance -1.0) 0.0 (Math|Float|SafeDivide _newtrack_0 5.0)) 0.0) false false))
          (if (.bBlockingHit (Collision|BreakHitResult _sweephitresult))
            (if (not (Variables|Default|GetbIsReversing))
              (Utilities|FlowControl|Sequence
                (:then_0
                  (Timeline|Timeline_1 Stop))
                (:then_1
                  (Utilities|FlowControl|Delay 2.0)
                  (Variables|Default|SetbIsReversing true)
                  (Timeline|Timeline_1 Reverse))))))
        (:Finished
          (if (Variables|Default|GetbIsReversing)
            (Variables|Default|SetbIsReversing false)
            (bind _output_get (Variables|Default|SetCrushCycleCount (+ (Variables|Default|GetCrushCycleCount) 1)))
            (if (>= _output_get 5)
              (goto _label Reset)
              (else
                (Utilities|FlowControl|Delay 3.0)
                (Timeline|Timeline_1 PlayFromStart)))
            (else
              (Variables|Default|SetbIsReversing true)
              (Utilities|FlowControl|Delay 2.0)
              (Timeline|Timeline_1 Reverse))))))))

(event EventTick
  (params (DeltaSeconds :type Float%20%28single-precision%29)))

(fn ConstructionScript)

(fn KillPlayer
  (params (HitActor :type Actor%20Object%20Reference))
  (bind _asbp_third_person_character (Utilities|Casting|CastToBP_ThirdPersonCharacter HitActor))
  (bind _output_get (Variables|/Game/ThirdPerson/Blueprints/BP_ThirdPersonCharacter.BP_ThirdPersonCharacter_C|SetLives _asbp_third_person_character (- (Variables|/Game/ThirdPerson/Blueprints/BP_ThirdPersonCharacter.BP_ThirdPersonCharacter_C|GetLives _asbp_third_person_character) 1)))
  (if (> _output_get 0)
    (Transformation|SetActorLocation _asbp_third_person_character (Variables|/Game/ThirdPerson/Blueprints/BP_ThirdPersonCharacter.BP_ThirdPersonCharacter_C|GetPlayerStartLocation _asbp_third_person_character) false false)
    (Physics|SetPhysicsLinearVelocity (Variables|/Script/Engine.MovementComponent|GetUpdatedPrimitive (Variables|/Script/Engine.Character|GetCharacterMovement _asbp_third_person_character)) "0, 0, 0" false "None")
    (else
      (bind _returnvalue (UserInterface|CreateWidget "/Game/UI/HUD_WBP.HUD_WBP_C"))
      (UserInterface|Viewport|AddtoViewport _returnvalue 0)
      (Game|SetGamePaused true))))