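; Hazard actor Blueprint that costs the third-person player a life when they overlap it.
; While lives remain, it teleports the character back to its stored start location and zeroes its physics velocity.
; When none remain, it shows the lose menu widget, switches to UI-only input with a mouse cursor and pauses the game.
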(event EventBeginPlay)

(event Collision|EventActorBeginOverlap
  (params (OtherActor :type Actor%20Object%20Reference))
  (bind _returnvalue (Game|GetPlayerController 0))
  (bind _asbp_third_person_character (Utilities|Casting|CastToBP_ThirdPersonCharacter OtherActor))
  (bind _output_get (Variables|/Game/ThirdPerson/Blueprints/BP_ThirdPersonCharacter.BP_ThirdPersonCharacter_C|SetLives _asbp_third_person_character (- (Variables|/Game/ThirdPerson/Blueprints/BP_ThirdPersonCharacter.BP_ThirdPersonCharacter_C|GetLives _asbp_third_person_character) 1)))
  (if (> _output_get 0)
    (Transformation|SetActorLocation _asbp_third_person_character (Variables|/Game/ThirdPerson/Blueprints/BP_ThirdPersonCharacter.BP_ThirdPersonCharacter_C|GetPlayerStartLocation _asbp_third_person_character) false false)
    (Physics|SetPhysicsLinearVelocity (Variables|/Script/Engine.MovementComponent|GetUpdatedPrimitive (Variables|/Script/Engine.Character|GetCharacterMovement _asbp_third_person_character)) "0, 0, 0" false "None")
    (else
      (bind _returnvalue_2 (UserInterface|CreateWidget "/Game/UI/LoseMenu_WBP.LoseMenu_WBP_C"))
      (UserInterface|Viewport|AddtoViewport _returnvalue_2 0)
      (Input|SetInputModeUIOnly _returnvalue 0 "DoNotLock" false)
      (Variables|/Script/Engine.PlayerController|SetbShowMouseCursor _returnvalue true)
      (Game|SetGamePaused true))))

(event EventTick
  (params (DeltaSeconds :type Float%20%28single-precision%29)))

(fn ConstructionScript)