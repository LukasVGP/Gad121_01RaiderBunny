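; Moving platform Blueprint that shuttles its mesh back and forth between StartPoint and EndPoint components.
; Tick advances or rewinds a clamped alpha by delta time over MoveDuration, lerps the mesh's relative location, and flips direction at either end.
; The construction script snaps the mesh to the start point.
; Despite the asset name, the Timeline and FlipFlop logic never runs; movement is entirely Tick-driven.
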(event EventBeginPlay)

(event Collision|EventActorBeginOverlap
  (params (OtherActor :type Actor%20Object%20Reference)))

(event EventTick
  (params (DeltaSeconds :type Float%20%28single-precision%29))
  (if (Variables|Default|GetbMovingForward)
    (Variables|Default|SetMoveAlpha (Math|Float|Clamp(Float) (+ (Variables|Default|GetMoveAlpha) (/ DeltaSeconds (Variables|Default|GetMoveDuration)))))
    (else
      (bind _output_get (Variables|Default|SetMoveAlpha (Math|Float|Clamp(Float) (- (Variables|Default|GetMoveAlpha) (/ DeltaSeconds (Variables|Default|GetMoveDuration))))))))
  (Transformation|SetRelativeLocation (Variables|Default|GetPlatformMesh) (Math|Vector|Lerp(Vector) (Variables|/Script/Engine.SceneComponent|GetRelativeLocation (Variables|Default|GetStartPoint)) (Variables|/Script/Engine.SceneComponent|GetRelativeLocation (Variables|Default|GetEndPoint)) _output_get) false false)
  (if (and (>= (Variables|Default|GetMoveAlpha) 1.0) (Variables|Default|GetbMovingForward))
    (Variables|Default|SetbMovingForward false))
  (if (and (<= (Variables|Default|GetMoveAlpha) 0.0) (not (Variables|Default|GetbMovingForward)))
    (Variables|Default|SetbMovingForward true)))

(fn ConstructionScript
  (Transformation|SetRelativeLocation (Variables|Default|GetPlatformMesh) (Variables|/Script/Engine.SceneComponent|GetRelativeLocation (Variables|Default|GetStartPoint)) false false))